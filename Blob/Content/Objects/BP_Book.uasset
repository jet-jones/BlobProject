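; BP_Book is a usable book object that shows its text to the player on screen.
; Its UseObject event creates a WB_Book widget, fills it with the book's Title and Content variables, and adds it to the viewport.
; It then casts the player character to BP_Player and switches it into UI mode.
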(event `self.UseObject`
  (params (HoveredObject :type "/Game/Objects/BP_BaseInteractableObject Object Reference"))
  (bind _returnvalue (`|CreateWidget` "/Game/Objects/WB_Book.WB_Book_C"))
  (set `TextBlock.Text` (`self.Content`) (`/Game/Objects/WB_Book.ContentText` _returnvalue))
  (set `TextBlock.Text` (`self.Title`) (`/Game/Objects/WB_Book.TitleText` _returnvalue))
  (`UserWidget.AddToViewport` _returnvalue 0)
  (bind _asbp_player (cast `/Game/Player/BP_Player` (`GameplayStatics.GetPlayerCharacter` 0)))
  (`/Game/Player/BP_Player.SetUIMode` _asbp_player true))

(fn `UserConstructionScript`
  (`parent.UserConstructionScript`))