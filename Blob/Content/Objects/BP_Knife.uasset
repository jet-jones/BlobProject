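; BP_Knife is a usable knife object that produces blob chunks when used on a blob.
; Its UseObject event continues only if the hovered object is a BP_Blob, then spawns a BP_BlobChunk at the first-person character's SafeSpawnLocation component.
; The blob itself is left unchanged, and the default BeginPlay, overlap and Tick events are disabled.
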(event `self.UseObject`
  (params (HoveredObject :type "/Game/Objects/BP_Object Object Reference"))
  (cast `/Game/Blob/BP_Blob` HoveredObject)
  (bind _asbp_first_person_character (cast `/Game/Player/BP_FirstPersonCharacter` (`GameplayStatics.GetPlayerCharacter` 0)))
  (`|SpawnActorFromClass` "/Game/Objects/BP_BlobChunk.BP_BlobChunk_C" (`KismetMathLibrary.MakeTransform` (`SceneComponent.K2_GetComponentLocation` (`/Game/Player/BP_FirstPersonCharacter.SafeSpawnLocation` _asbp_first_person_character))) "Undefined" "MultiplyWithRoot" null null))

(fn `UserConstructionScript`
  (`parent.UserConstructionScript`))