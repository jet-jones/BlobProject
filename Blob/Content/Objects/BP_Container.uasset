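; BP_Container is a holder object that receives a held object and places it at a fixed offset.
; It overrides GivenHeldObject, calls the parent version, then prints a debug message.
; The received actor is moved to the ObjectOffset component's world location and attached to the container, keeping its world transform.
; The event graph and construction script add no behavior of their own.
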(fn `GivenHeldObject`
  (params (HeldObject :type "/Game/Objects/BP_Object Object Reference"))
  (returns (Success :type Boolean))
  (bind _success (`parent.GivenHeldObject` HeldObject))
  (`KismetSystemLibrary.PrintString` "Given Object")
  (`self.K2_SetActorLocation` (`local.HeldObject`) (`SceneComponent.K2_GetComponentLocation` (`self.ObjectOffset`)) false false)
  (`self.K2_AttachToActor` (`local.HeldObject`) self "None" "KeepWorld" "KeepWorld" "KeepWorld" false)
  (return _success))

(fn `UserConstructionScript`
  (`parent.UserConstructionScript`))