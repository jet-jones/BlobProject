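; BP_Plate is a plate object that can receive one held item from another actor.
; GivenHeldObject checks for attached actors; if none, it teleports the item to the ObjectOffset component, attaches it keeping world transform, and returns true.
; If something is already attached, it prints a message and returns false.
; The UseObject event is present but empty, and the other graph events are unused.
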(event `self.UseObject`
  (params (HoveredObject :type "/Game/Objects/BP_Object Object Reference")))

(fn `GivenHeldObject`
  (params (HeldObject :type "/Game/Objects/BP_Object Object Reference"))
  (returns (Success :type Boolean))
  (if (== (`KismetArrayLibrary.Array_Length` (`self.GetAttachedActors` true)) 0)
    (`self.K2_SetActorLocation` (`local.HeldObject`) (`SceneComponent.K2_GetComponentLocation` (`self.ObjectOffset`)) false false)
    (`self.K2_AttachToActor` (`local.HeldObject`) self "None" "KeepWorld" "KeepWorld" "KeepWorld" false)
    (return true)
    (else
      (`KismetSystemLibrary.PrintString` "Can't put on plate because something is already there")
      (return false))))

(fn `UserConstructionScript`
  (`parent.UserConstructionScript`))