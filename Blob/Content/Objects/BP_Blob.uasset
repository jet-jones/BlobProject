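; BP_Blob is an object that pulls a BP_Book to its own position when it interacts with one.
; InteractwithOtherObject ignores anything that is not a BP_Book, then plays a timeline from the start.
; Each timeline update lerps the book from its current location toward the blob by the track value, moving it without sweep.
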(event `self.InteractWithOtherObject`
  (params (Object :type "/Game/Objects/BP_Object Object Reference"))
  (bind _asbp_book (cast `/Game/Objects/BP_Book` Object))
  (bind (_direction _newtrack_0) (`Timeline|Timeline` :!via `PlayFromStart`)
    (:`Update`
      (`self.K2_SetActorLocation` _asbp_book (`KismetMathLibrary.VLerp` (`self.K2_GetActorLocation` _asbp_book) (`self.K2_GetActorLocation`) _newtrack_0) false false))))

(fn `UserConstructionScript`
  (`parent.UserConstructionScript`))