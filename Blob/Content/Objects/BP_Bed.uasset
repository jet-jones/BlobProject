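; BP_Bed is a usable bed object that lets the player sleep.
; On UseObject it casts the first player pawn to BP_Player and calls its Sleep, passing the mesh's world location as the sleep position and itself as the bed actor.
; The sleep behavior itself lives in the player, as the bed has no other active logic.
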(event `self.UseObject`
  (params (HoveredObject :type "/Game/Objects/BP_BaseInteractableObject Object Reference") (IsHeld :type Boolean))
  (bind _asbp_player (cast `/Game/Player/BP_Player` (`GameplayStatics.GetPlayerPawn` 0)))
  (`/Game/Player/BP_Player.Sleep` _asbp_player (`SceneComponent.K2_GetComponentLocation` (`self.Mesh`)) self null))

(fn `UserConstructionScript`
  (`parent.UserConstructionScript`))