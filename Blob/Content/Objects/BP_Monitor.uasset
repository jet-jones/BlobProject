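; BP_Monitor is a monitor actor whose display changes to match the object passed to its UpdateInputObject event.
; A BP_Microphone reveals the Widget component, while a BP_CameraTripod swaps the screen's mesh material to M_WorldCamera.
; An invalid input resets both by restoring M_Blob and hiding the widget.
; Switching directly between valid inputs does not clear the previous state.
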(event `UpdateInputObject`
  (params (Object :type "/Game/Objects/BP_BaseInteractableObject Object Reference"))
  (`/Engine/EditorBlueprintResources/StandardMacros.IsValid` Object
    (:`Is Valid`
      (cast `/Game/Objects/BP_Microphone` Object
        (:`then`
          (`SceneComponent.SetVisibility` (`self.Widget`) true false))
        (:`CastFailed`
          (cast `/Game/Objects/BP_CameraTripod` Object)
          (`PrimitiveComponent.SetMaterial` (`self.Mesh`) 1 "/Game/Objects/M_WorldCamera.M_WorldCamera"))))
    (:`Is Not Valid`
      ;[1 1 1] Everything must get reset here
      (`PrimitiveComponent.SetMaterial` (`self.Mesh`) 1 "/Game/Blob/M_Blob.M_Blob")
      (`SceneComponent.SetVisibility` (`self.Widget`) false false))))

(fn `UserConstructionScript`)