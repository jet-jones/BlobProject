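; BP_Photo is a photo object that displays a render target texture on its Cube1 component.
; On BeginPlay it creates a dynamic material instance for the first material slot and assigns the RenderTarget variable to its Diffuse texture parameter.
; Tick and the construction script only call the parent implementation, and the overlap event is disabled.
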(event `self.ReceiveBeginPlay`
  (bind _cube1 (`self.Cube1`))
  (`parent.ReceiveBeginPlay`)
  (bind _returnvalue (`PrimitiveComponent.CreateDynamicMaterialInstance` _cube1 0 null "None"))
  (`PrimitiveComponent.SetMaterial` _cube1 0 _returnvalue)
  (`MaterialInstanceDynamic.SetTextureParameterValue` _returnvalue "Diffuse" (`self.RenderTarget`)))

(event `self.ReceiveTick`
  (params (DeltaSeconds :type "Float (single-precision)"))
  (`parent.ReceiveTick` DeltaSeconds))

(fn `UserConstructionScript`
  (`parent.UserConstructionScript`))