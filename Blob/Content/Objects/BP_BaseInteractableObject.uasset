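; BP_BaseInteractableObject is a base Blueprint for objects the player can interact with.
; On BeginPlay it caches the Mesh's default material and a reference to BP_Player.
; Fire marks the object burnt once and puts a burnt material on every static mesh component.
; Use, stop-using, pickup and drop events are empty stubs, GivenHeldObject returns false, and a hover-highlight material swap is left disconnected.
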(event `self.ReceiveBeginPlay`
  (set `self.DefaultMaterial` (`PrimitiveComponent.GetMaterial` (`self.Mesh`) 0))
  (bind _asbp_player (cast `/Game/Player/BP_Player` (`GameplayStatics.GetPlayerCharacter` 0)))
  (set `self.Player` _asbp_player))

(event `self.ReceiveTick`
  (params (DeltaSeconds :type "Float (single-precision)")))

(event `Fire`
  (if (not (`self.IsBurnt`))
    (set `self.IsBurnt` true)
    (for _array_element (`self.K2_GetComponentsByClass` "/Script/Engine.StaticMeshComponent")
      (`PrimitiveComponent.SetMaterial` _array_element 0 "/Game/Objects/M_BurntMaterial.M_BurntMaterial"))))

(event `UseObject`
  (params (HoveredObject :type "/Game/Objects/BP_BaseInteractableObject Object Reference") (IsHeld :type Boolean)))

(event `StopUsingObject`)

(event `PickupObject`)

(event `DropObject`)

(fn `GivenHeldObject`
  (params (HeldObject :type "/Game/Objects/BP_BaseInteractableObject Object Reference"))
  (returns (Success :type Boolean))
  (return false))

(fn `UserConstructionScript`)