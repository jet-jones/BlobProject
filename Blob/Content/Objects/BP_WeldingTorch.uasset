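; Usable welding torch that burns interactable objects it is pointed at.
; Use and stop events toggle the torch's Niagara effect and an in-use flag.
; While in use, each Tick line-traces along the effect's up vector, with debug drawing left on, and calls Burnt on any BP_BaseInteractableObject hit.
; A branch that would weld BP_Tape is present but disconnected.
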(event `self.ReceiveTick`
  (params (DeltaSeconds :type "Float (single-precision)"))
  (bind _returnvalue (`SceneComponent.K2_GetComponentLocation` (`self.NS_WeldingTorch`)))
  (`parent.ReceiveTick` DeltaSeconds)
  (if (`self.is_using`)
    (bind _outhit (`KismetSystemLibrary.LineTraceSingle` :`Start` _returnvalue :`End` (+ _returnvalue (* (`SceneComponent.GetUpVector` (`self.NS_WeldingTorch`)) 5000.0)) :`TraceChannel` "TraceTypeQuery1" :`DrawDebugType` "ForDuration" :`DrawTime` 1.0))
    (bind _asbp_base_interactable_object (cast `/Game/Objects/BP_BaseInteractableObject` (`.HitActor` (`GameplayStatics.BreakHitResult` _outhit))))
    (`self.Burnt` _asbp_base_interactable_object)))

(event `self.UseObject`
  (params (HoveredObject :type "/Game/Objects/BP_BaseInteractableObject Object Reference"))
  (`ActorComponent.SetActive` (`self.NS_WeldingTorch`) true false)
  (set `self.is_using` true))

(event `self.StopUsingObject`
  (`ActorComponent.SetActive` (`self.NS_WeldingTorch`) false false)
  (set `self.is_using` false))

(fn `UserConstructionScript`
  (`parent.UserConstructionScript`))