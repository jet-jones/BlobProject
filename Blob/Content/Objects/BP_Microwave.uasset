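; Interactable microwave that holds certain held objects and cooks them while its door is shut.
; UseObject toggles the door, and Tick eases the mesh yaw between open and closed.
; GivenHeldObject matches a hardcoded class whitelist, then moves the item to the Arrow and attaches it.
; After a short closed-door timer, Tick calls Fire every frame on all attached interactable objects, and opening the door resets the timer.
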(event `self.ReceiveTick`
  (params (DeltaSeconds :type "Float (single-precision)"))
  (bind _staticmesh (`self.StaticMesh`))
  (bind (_relativerotation_roll _relativerotation_pitch _relativerotation_yaw) (`KismetMathLibrary.BreakRotator` (`SceneComponent.RelativeRotation` _staticmesh)))
  (`parent.ReceiveTick` DeltaSeconds)
  (`SceneComponent.K2_SetRelativeRotation` _staticmesh (`KismetMathLibrary.MakeRotator` 0.0 0.0 (`KismetMathLibrary.Lerp` _relativerotation_yaw (`KismetMathLibrary.SelectFloat` 100.0 0.0 (`self.DoorOpen`)) 0.4)) false false)
  (if (`self.DoorOpen`)
    (set `self.Timer` 0.0)
    (else
      (bind _output_get (set `self.Timer` (+ (`self.Timer`) (`GameplayStatics.GetWorldDeltaSeconds`))))
      (if (> _output_get 2.0)
        (for _array_element (`self.GetAttachedActors` true true)
          (bind _asbp_base_interactable_object (cast `/Game/Objects/BP_BaseInteractableObject` _array_element))
          (`self.Fire` _asbp_base_interactable_object))))))

(event `self.UseObject`
  (params (HoveredObject :type "/Game/Objects/BP_BaseInteractableObject Object Reference") (IsHeld :type Boolean))
  (set `self.DoorOpen` (not (`self.DoorOpen`))))

(fn `GivenHeldObject`
  (params (HeldObject :type "/Game/Objects/BP_BaseInteractableObject Object Reference"))
  (returns (Success :type Boolean))
  (bind _heldobject (`local.HeldObject`))
  (`parent.GivenHeldObject` HeldObject)
  (for _array_element (`|MakeArray` "/Game/Objects/BP_Wire.BP_Wire_C" "/Game/Objects/BP_Book.BP_Book_C" "/Game/Objects/BP_BlobChunk.BP_BlobChunk_C" "/Game/Objects/BP_Battery.BP_Battery_C" "/Game/Objects/BP_Plant.BP_Plant_C" "/Game/Objects/BP_Tape.BP_Tape_C" "/Game/Objects/BP_Knife.BP_Knife_C" "/Game/Objects/BP_Camera.BP_Camera_C" "/Game/Objects/BP_Plate.BP_Plate_C" "/Game/Objects/BP_WeldingTorch.BP_WeldingTorch_C" :!type "/Game/Objects/BP_BaseInteractableObject Class Reference")
    (if (== _array_element (`GameplayStatics.GetObjectClass` HeldObject))
      (`self.K2_SetActorLocation` _heldobject (`SceneComponent.K2_GetComponentLocation` (`self.Arrow`)) false false)
      (`self.K2_AttachToActor` _heldobject self "None" "KeepWorld" "SnapToTarget" "KeepWorld" true)
      (return true))))

(fn `UserConstructionScript`
  (`parent.UserConstructionScript`))